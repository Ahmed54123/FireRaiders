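; BP_Interaction is a configurable interactive skeletal-mesh prop in the Fire Equipment Bundle that toggles between two animated states.
; Each Interact event flips between two animations with matching sounds played at the Sphere's location; only the first animation can loop.
; The construction script applies the chosen mesh and sets the Sphere's scale and position from variables, so one Blueprint can serve different props.
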(event `Interact`
  (bind _skeletalmesh (`self.SkeletalMesh`))
  (bind _returnvalue (`SceneComponent.K2_GetComponentLocation` (`self.Sphere`)))
  (`/Engine/EditorBlueprintResources/StandardMacros.FlipFlop`
    (:`A`
      (`SkeletalMeshComponent.PlayAnimation` _skeletalmesh (`self.Anim1`) (`self.AnimLooping`))
      (`GameplayStatics.PlaySoundAtLocation` (`self.Sound1`) _returnvalue (struct) 1.0 1.0 0.0 null null null null))
    (:`B`
      (`SkeletalMeshComponent.PlayAnimation` _skeletalmesh (`self.Anim2`) false)
      (`GameplayStatics.PlaySoundAtLocation` (`self.Sound2`) _returnvalue (struct) 1.0 1.0 0.0 null null null null))))

(fn `UserConstructionScript`
  (bind _sphere (`self.Sphere`))
  (`SkinnedMeshComponent.SetSkinnedAssetAndUpdate` (`self.SkeletalMesh`) (`self.Mesh`) true)
  (`SceneComponent.SetWorldScale3D` _sphere (`self.TriggerRadius`))
  (`SceneComponent.K2_SetRelativeLocation` _sphere (`self.TriggerLocation`) false false))
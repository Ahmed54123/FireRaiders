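; Interaction component for Fire_Fight that shows or hides a UI prompt for interactable objects.
; DisplayWidgetOnOverlap stores the pressed state and toggles UiPrompt visibility only for actors implementing I_player, and only while the button is unpressed.
; DisplayUi sets the prompt's visibility directly, without those checks.
; Overlap detection is left to callers, as BeginPlay and Tick are unused.
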(fn `display ui`
  (params (OnOff :type Boolean))
  (`SceneComponent.SetVisibility` (`self.ui prompt`) (select `bool` OnOff :`true` true) false))

(fn `display widget on overlap`
  (params (`other actor` :type "Actor Object Reference") (pressed :type Boolean) (onOff :type Boolean))
  (locals (pressedButton :type Boolean :default false))
  (set `local.pressedButton` pressed)
  (if (`KismetSystemLibrary.DoesImplementInterface` `other actor` "/Game/Fire_Fight/Characters/main_char/i_player.i_player_C")
    (if (not (`local.pressedButton`))
      (`SceneComponent.SetVisibility` (`self.ui prompt`) (select `bool` onOff :`true` true) false))))
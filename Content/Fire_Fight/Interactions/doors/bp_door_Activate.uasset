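; Door actor that stays locked until externally activated, then loads the next level when the player interacts with it.
; An overlap sphere shows the interact widget through BpcInteract when unlocked, or sends locked-door text to actors implementing I_player, and clears both on exit.
; ActivateFunction unlocks the door and swaps its material, while Interact marks it opened and opens the NextLevel reference.
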(event `self.overlapSphere.OnComponentBeginOverlap`
  (params (OverlappedComponent :type "PrimitiveComponent Object Reference") (OtherActor :type "Actor Object Reference") (OtherComp :type "PrimitiveComponent Object Reference") (OtherBodyIndex :type Integer) (bFromSweep :type Boolean) (SweepResult :type "HitResult Structure (by ref)"))
  (if (`self.door unlocked`)
    (`/Game/Fire_Fight/Interactions/bpc_interact.display widget on overlap` (`self.bpc_interact`) OtherActor (`self.opened`) true)
    (elif (`KismetSystemLibrary.DoesImplementInterface` OtherActor "/Game/Fire_Fight/Characters/main_char/i_player.i_player_C")
      (message `/Game/Fire_Fight/Characters/main_char/i_player.set text` OtherActor (`self.locked door text`)))))

(event `self.overlapSphere.OnComponentEndOverlap`
  (params (OverlappedComponent :type "PrimitiveComponent Object Reference") (OtherActor :type "Actor Object Reference") (OtherComp :type "PrimitiveComponent Object Reference") (OtherBodyIndex :type Integer))
  (`/Game/Fire_Fight/Interactions/bpc_interact.display widget on overlap` (`self.bpc_interact`) OtherActor (`self.opened`) false)
  (message `/Game/Fire_Fight/Characters/main_char/i_player.set text` OtherActor ""))

(event `/Game/Fire_Fight/Interactions/I_Interact.Interact`
  (if (`self.door unlocked`)
    (set `self.opened` true)
    (`GameplayStatics.OpenLevelBySoftObjectPtr` (`self.next Level`))))

(event `/Game/Fire_Fight/Interactions/I_Activated.ActivateFunction`
  (set `self.door unlocked` true)
  (`PrimitiveComponent.SetMaterial` (`self.door`) 0 "/Engine/MapTemplates/Materials/BasicAsset03.BasicAsset03"))

(fn `UserConstructionScript`
  (`parent.UserConstructionScript`))
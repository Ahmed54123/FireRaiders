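; Interactable door for Fire_Fight that loads the level set in NextLevel when the player interacts with it.
; An overlap sphere shows or hides the prompt through the BpcInteract component, passing along the door's Opened state.
; Interact marks the door opened and opens the level by object reference.
; The construction script copies the door's prompt text into the component and hides its UI by default.
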(event `self.overlapSphere.OnComponentBeginOverlap`
  (params (OverlappedComponent :type "PrimitiveComponent Object Reference") (OtherActor :type "Actor Object Reference") (OtherComp :type "PrimitiveComponent Object Reference") (OtherBodyIndex :type Integer) (bFromSweep :type Boolean) (SweepResult :type "HitResult Structure (by ref)"))
  (`/Game/Fire_Fight/Interactions/bpc_interact.display widget on overlap` (`self.bpc_interact`) OtherActor (`self.opened`) true))

(event `self.overlapSphere.OnComponentEndOverlap`
  (params (OverlappedComponent :type "PrimitiveComponent Object Reference") (OtherActor :type "Actor Object Reference") (OtherComp :type "PrimitiveComponent Object Reference") (OtherBodyIndex :type Integer))
  (`/Game/Fire_Fight/Interactions/bpc_interact.display widget on overlap` (`self.bpc_interact`) OtherActor (`self.opened`) false))

(event `/Game/Fire_Fight/Interactions/I_Interact.Interact`
  (set `self.opened` true)
  (`GameplayStatics.OpenLevelBySoftObjectPtr` (`self.next Level`)))

(fn `UserConstructionScript`
  (bind _bpc_interact (`self.bpc_interact`))
  (set `/Game/Fire_Fight/Interactions/bpc_interact.ui prompt` (`self.interactPrompt`) _bpc_interact)
  (`/Game/Fire_Fight/Interactions/bpc_interact.display ui` _bpc_interact false))
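; BP_Button is an interactable button that activates a list of target actors when pressed.
; Interact latches Pressed, sends the activate message to each target, plays optional click text and hides the prompt; reusable buttons reset after a delay.
; Prompt overlaps drive the widget through BpcInteractCOMP, which receives WPrompt in the construction script.
; Tick polls Pressed to swap the button material and hide the interact effect.
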(event `self.ReceiveTick`
  (params (DeltaSeconds :type "Float (single-precision)"))
  (`|ExecutionSequence`
    (:`then_0`
      (`SceneComponent.SetHiddenInGame` (`self.InteractEffect`) (`self.Pressed`) true)
      (`PrimitiveComponent.SetMaterial` (`self.butt`) 0 (select `bool` (`self.Pressed`) :`false` "/Game/Fire_Fight/imports/mixamo/characters/main_v1/Wolf3D_Glasses.Wolf3D_Glasses" :`true` "/Game/starter_content_stuff/StarterContent/Materials/M_Basic_Wall.M_Basic_Wall" :!type "MaterialInterface Object Reference")))))

(event `/Game/Fire_Fight/Interactions/I_Interact.Interact`
  (if (not (`self.Pressed`))
    (set `self.Pressed` true)
    (`|ExecutionSequence`
      (:`then_0`
        (if (`self.JuiceOn`)
          (`ActorComponent.Activate` (`self.click text`) false)))
      (:`then_1`
        (for _array_element (`self.ActivateTarget`)
          (message `/Game/Fire_Fight/Interactions/I_Activated.ActivateFunction` _array_element))
        (if (`self.Reusable`)
          (`KismetSystemLibrary.Delay` (`self.ButtonWaitTime`))
          (set `self.Pressed` false)))
      (:`then_2`
        (`/Game/Fire_Fight/Interactions/bpc_interact.display ui` (`self.bpc_interactCOMP`) false)))))

(event `self.prompt.OnComponentBeginOverlap`
  (params (OverlappedComponent :type "PrimitiveComponent Object Reference") (OtherActor :type "Actor Object Reference") (OtherComp :type "PrimitiveComponent Object Reference") (OtherBodyIndex :type Integer) (bFromSweep :type Boolean) (SweepResult :type "HitResult Structure (by ref)"))
  (`/Game/Fire_Fight/Interactions/bpc_interact.display widget on overlap` (`self.bpc_interactCOMP`) OtherActor (`self.Pressed`) true))

(event `self.prompt.OnComponentEndOverlap`
  (params (OverlappedComponent :type "PrimitiveComponent Object Reference") (OtherActor :type "Actor Object Reference") (OtherComp :type "PrimitiveComponent Object Reference") (OtherBodyIndex :type Integer))
  (`/Game/Fire_Fight/Interactions/bpc_interact.display widget on overlap` (`self.bpc_interactCOMP`) OtherActor (`self.Pressed`) false))

(fn `UserConstructionScript`
  (set `/Game/Fire_Fight/Interactions/bpc_interact.ui prompt` (`self.w_prompt`) (`self.bpc_interactCOMP`)))
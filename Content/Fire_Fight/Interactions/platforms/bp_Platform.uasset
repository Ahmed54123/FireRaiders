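; Moving platform Blueprint that continuously shuttles a platform between its starting transform and a hidden target marker.
; The construction script caches the start transform, and BeginPlay hides the TargetActor component and applies Speed as the timeline play rate.
; Tick starts the MovePlatform timeline whenever idle, interpolating location and rotation while keeping the start scale.
; Each finish flips Loop, which acts as a direction flag alternating forward and reverse playback.
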(event `self.ReceiveBeginPlay`
  (`|ExecutionSequence`
    (:`then_0`
      (`SceneComponent.SetVisibility` (`self.target actor`) false false))
    (:`then_1`
      (`TimelineComponent.SetPlayRate` (`self.Move platform`) (`self.Speed`)))))

(event `self.ReceiveTick`
  (params (DeltaSeconds :type "Float (single-precision)"))
  (bind _start_transform (`self.start transform`))
  (if (not (`self.isPlaying`))
    (if (not (`self.loop?`))
      (bind (_direction _move_platform) (`Timeline|Move platform` :!label _label)
        (:`Update`
          (set `self.isPlaying` true)
          (`SceneComponent.K2_SetWorldTransform` (`self.platform`) (`KismetMathLibrary.TLerp` _start_transform (`KismetMathLibrary.MakeTransform` (.location (`SceneComponent.K2_GetComponentToWorld` (`self.target actor`))) (.rotation (`SceneComponent.K2_GetComponentToWorld` (`self.target actor`))) (.scale _start_transform)) _move_platform) false false))
        (:`Finished`
          (`self.End timeline`)))
      (else
        (goto _label :!via `ReverseFromEnd`)))))

(fn `UserConstructionScript`
  (set `self.start transform` (`SceneComponent.K2_GetComponentToWorld` (`self.platform`))))
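; BP_WireSpline is a spline-shaped electrical wire in the Fire_Fight wire puzzle that can be de-electrified.
; The construction script adds a Z-forward spline mesh per segment and passes the spline to a Niagara electricity effect.
; ActivateFunction deactivates that effect and sets the de-electrified material on the spline component itself, indexed by point, rather than on the generated meshes.
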(event `self.ReceiveBeginPlay`)

(event `/Game/Fire_Fight/Interactions/I_Activated.ActivateFunction`
  (bind _spline (`self.Spline`))
  (`ActorComponent.Deactivate` (`self.nS_ElectricitySM1`))
  (for _index (range (`SplineComponent.GetNumberOfSplinePoints` _spline))
    (`PrimitiveComponent.SetMaterial` _spline _index "/Game/Fire_Fight/Interactions/WirePuzzle/M_DeElectric.M_DeElectric")))

(fn `UserConstructionScript`
  (bind _spline (`self.Spline`))
  (for _index (range (+ (- (`SplineComponent.GetNumberOfSplinePoints` (`self.Spline`)) 2) 1))
    (bind _returnvalue (`AddComponent|NODE_AddSplineMeshComponent-0`))
    (`SplineMeshComponent.SetForwardAxis` _returnvalue "Z" true)
    (bind _returnvalue_2 (+ _index 1))
    (`SplineMeshComponent.SetStartAndEnd` _returnvalue (`SplineComponent.GetLocationAtSplinePoint` _spline _index "Local") (`SplineComponent.GetTangentAtSplinePoint` _spline _index "Local") (`SplineComponent.GetLocationAtSplinePoint` _spline _returnvalue_2 "Local") (`SplineComponent.GetTangentAtSplinePoint` _spline _returnvalue_2 "Local") true)
    (`NiagaraComponent.SetNiagaraVariableObject` (`self.nS_ElectricitySM1`) "New Spline" (`self.Spline`))))
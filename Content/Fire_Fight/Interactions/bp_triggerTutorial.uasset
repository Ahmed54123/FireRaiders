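; A tutorial trigger Blueprint for Fire_Fight that hides its Cube at BeginPlay and unpauses the game on IA_Interact if its TutorialPaused flag is set.
; Disconnected logic would check an actor for I_player, send a tutorial message through BP_GameManager, pause the game and set that flag.
; The ActorBeginOverlap event is empty, so nothing in this graph currently starts the tutorial pause.
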(event `self.ReceiveBeginPlay`
  (`SceneComponent.SetHiddenInGame` (`self.Cube`) true false))

(event `self.ReceiveActorBeginOverlap`
  (params (OtherActor :type "Actor Object Reference")))

(event `EnhancedInput|/Game/ThirdPerson/Input/Actions/IA_Interact`
  (params (ActionValue :type Boolean) (ElapsedSeconds :type "Float (double-precision)") (TriggeredSeconds :type "Float (double-precision)") (InputAction :type "InputAction Object Reference" :default "/Game/ThirdPerson/Input/Actions/IA_Interact.IA_Interact"))
  (:`Started`
    (if (`self.TutorialPaused`)
      (`GameplayStatics.SetGamePaused` false)
      (set `self.TutorialPaused` false))))

(fn `UserConstructionScript`)
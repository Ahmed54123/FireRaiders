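; A trigger volume that shows a configurable text message to the player while they stand inside it.
; Its Cube is hidden when play begins, leaving an invisible overlap area.
; On begin overlap, actors implementing I_player receive TextToSet through SetTextMessage, and on end overlap they receive an empty string to clear it.
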(event `self.ReceiveBeginPlay`
  (`SceneComponent.SetHiddenInGame` (`self.Cube`) true false))

(event `self.ReceiveActorBeginOverlap`
  (params (OtherActor :type "Actor Object Reference"))
  (if (`KismetSystemLibrary.DoesImplementInterface` OtherActor "/Game/Fire_Fight/Characters/main_char/i_player.i_player_C")
    (message `/Game/Fire_Fight/Characters/main_char/i_player.set text` OtherActor (`self.text to set`))))

(event `self.ReceiveActorEndOverlap`
  (params (OtherActor :type "Actor Object Reference"))
  (if (`KismetSystemLibrary.DoesImplementInterface` OtherActor "/Game/Fire_Fight/Characters/main_char/i_player.i_player_C")
    (message `/Game/Fire_Fight/Characters/main_char/i_player.set text` OtherActor "")))

(fn `UserConstructionScript`)
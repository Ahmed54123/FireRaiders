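; BP_socketMoveable is a carryable, burnable prop in the fire-fighting game that shows an interact prompt.
; StartBurning spawns fire on the cube's fire socket through BPCBurnableProperties.
; TakeDamage scales damage by the fire multiplier into BPCDamageable, throttled by brief invulnerability; on death it applies a burnt material, puts out the fire and hides the prompt.
; BpcInteract toggles the prompt on overlap, Carry and PutDown.
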(event `self.ReceiveTick`
  (params (DeltaSeconds :type "Float (single-precision)")))

(event `/Game/Fire_Fight/I_idamageable.takeDamage`
  (params (damage :type "Float (double-precision)"))
  (bind _bpc_burnableproperties (`self.BPC_BurnableProperties`))
  ;[1 1 1] fire properties
  (if (not (`self.invulnerable`))
    (`/Game/Fire_Fight/BPC_damageable.TakeDamageFunc` (`self.BPC_damageable`) (* damage (`/Game/Fire_Fight/Fire_Fire/BPC_BurnableProperties.fireEffectMultiplier` (`self.BPC_BurnableProperties`))))
    (set `self.invulnerable` true)
    (`KismetSystemLibrary.Delay` 0.1)
    (set `self.invulnerable` false)
    (if (`/Game/Fire_Fight/BPC_damageable.isDead` (`self.BPC_damageable`))
      (`PrimitiveComponent.SetMaterial` (`self.Cube`) 0 "/Game/Fire_Fight/Materials/M_BurntObject.M_BurntObject")
      (if (not (`/Game/Fire_Fight/Fire_Fire/BPC_BurnableProperties.ObjectBurnt` _bpc_burnableproperties))
        (message `/Game/Fire_Fight/Fire_Fire/I_Burnable.FireDieOut` (`/Game/Fire_Fight/Fire_Fire/BPC_BurnableProperties.FireSpawn` _bpc_burnableproperties))
        (set `/Game/Fire_Fight/Fire_Fire/BPC_BurnableProperties.ObjectBurnt` true _bpc_burnableproperties)
        (`/Game/Fire_Fight/Interactions/bpc_interact.display ui` (`self.bpc_interact`) false)))))

(event `/Game/Fire_Fight/Fire_Fire/I_Burnable.Start Burning`
  (params (`fire type` :type "/Game/Fire_Fight/Fire_Fire/fire_variants/e_FireType Enum" :default "NewEnumerator0") (`Spread Rate multiplier` :type "Float (double-precision)"))
  ;[1 1 1] fire properties
  (`/Game/Fire_Fight/Fire_Fire/BPC_BurnableProperties.SpawnFire` :`self` (`self.BPC_BurnableProperties`) :`FireLocation` (`self.Cube`) :`socket name` "fire socket" :`fire type` `fire type`))

(event `self.outlineEffect.OnComponentBeginOverlap`
  (params (OverlappedComponent :type "PrimitiveComponent Object Reference") (OtherActor :type "Actor Object Reference") (OtherComp :type "PrimitiveComponent Object Reference") (OtherBodyIndex :type Integer) (bFromSweep :type Boolean) (SweepResult :type "HitResult Structure (by ref)"))
  ;[1 1 1] outline char
  (`/Game/Fire_Fight/Interactions/bpc_interact.display widget on overlap` (`self.bpc_interact`) OtherActor false true))

(event `self.outlineEffect.OnComponentEndOverlap`
  (params (OverlappedComponent :type "PrimitiveComponent Object Reference") (OtherActor :type "Actor Object Reference") (OtherComp :type "PrimitiveComponent Object Reference") (OtherBodyIndex :type Integer))
  ;[1 1 1] outline char
  (`/Game/Fire_Fight/Interactions/bpc_interact.display widget on overlap` (`self.bpc_interact`) OtherActor false false))

(event `/Game/Fire_Fight/Interactions/I_holdable.carry`
  (`/Game/Fire_Fight/Interactions/bpc_interact.display ui` (`self.bpc_interact`) false))

(event `/Game/Fire_Fight/Interactions/I_holdable.put down`
  (`/Game/Fire_Fight/Interactions/bpc_interact.display ui` (`self.bpc_interact`) true))

(fn `GetBurnRate`
  (returns (`Burn Rate` :type "Float (double-precision)"))
  (return 0.0))

(fn `GetMaterial`
  (returns (`Structure Type` :type "/Game/Fire_Fight/Fire_Fire/E_MaterialTypes Enum"))
  (return "NewEnumerator0"))

(fn `UserConstructionScript`
  (`MeshComponent.SetOverlayMaterial` (`self.Cube`) null)
  (set `/Game/Fire_Fight/Interactions/bpc_interact.ui prompt` (`self.Widget`) (`self.bpc_interact`)))
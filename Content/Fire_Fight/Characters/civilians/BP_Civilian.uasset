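; Rescuable civilian that the player carries to a safe point before it dies, reporting its spawn, rescue and death to BP_GameManager.
; Overlapping an I_civSafePoint actor attaches it, plays a cheer and later hides it.
; BPCDamageable tracks health, which Tick feeds to the W_CivUI marker while polling for death, calling CivilianDie every frame once dead.
; Overlap spheres drive interaction prompts and cue-indexed dialogue; carry and put-down work, while throwing is disabled.
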(event `/Game/Fire_Fight/I_idamageable.takeDamage`
  (params (damage :type "Float (double-precision)"))
  ;[1 0.09711 0] take damage
  (`/Game/Fire_Fight/BPC_damageable.TakeDamageFunc` (`self.BPC_damageable`) damage))

(event `/Game/Fire_Fight/Characters/civilians/I_Civilian.CivilianSaved`
  (bind _sphere (`self.Sphere`))
  ;[0.6382 1 0] civilian saved effects
  (`KismetSystemLibrary.PrintString` "he got saved")
  (set `self.CivilianSafe` true)
  (`PrimitiveComponent.SetSimulatePhysics` _sphere false)
  (`PrimitiveComponent.SetCollisionEnabled` _sphere "NoCollision")
  (`SceneComponent.SetVisibility` (`self.checpoint widget`) false false)
  (`self.play dialogue` 3)
  (bind _returnvalue (`GameplayStatics.GetActorOfClass` "/Game/Fire_Fight/Assets/BP_GameManager.BP_GameManager_C"))
  (message `/Game/Fire_Fight/I_GameManager.CivilianSaved` _returnvalue)
  (`SceneComponent.K2_DetachFromComponent` (`self.Sphere`) "KeepWorld" "KeepRelative" "KeepWorld" true))

(event `self.ReceiveBeginPlay`
  ;[0.02258 0.5161 1] add to game manager
  (bind _returnvalue (`GameplayStatics.GetActorOfClass` "/Game/Fire_Fight/Assets/BP_GameManager.BP_GameManager_C"))
  (message `/Game/Fire_Fight/I_GameManager.AddCivilian` _returnvalue)
  (if (not (`self.juiceON`))
    ;[1 0.5615 0] setup widget
    (`SceneComponent.SetVisibility` (`self.checpoint widget`) false false)))

(event `self.ReceiveTick`
  (params (DeltaSeconds :type "Float (single-precision)"))
  (bind _bpc_damageable (`self.BPC_damageable`))
  (bind _sphere (`self.Sphere`))
  (bind _returnvalue (`WidgetComponent.GetWidget` (`self.checpoint widget`)))
  (bind (_relativerotation_roll _relativerotation_pitch _relativerotation_yaw) (`KismetMathLibrary.BreakRotator` (`SceneComponent.RelativeRotation` _sphere)))
  (`|ExecutionSequence`
    (:`then_0`
      ;[1 0.6412 0] widget sets
      (`/Engine/EditorBlueprintResources/StandardMacros.IsValid` _returnvalue
        (:`Is Valid`
          (bind _asw_civ_ui (cast `/Game/Fire_Fight/joost/civilians_UI/W_CivUI` _returnvalue))
          (set `/Game/Fire_Fight/joost/civilians_UI/W_CivUI.origin location` (`self.K2_GetActorLocation`) _asw_civ_ui)
          (set `/Game/Fire_Fight/joost/civilians_UI/W_CivUI.health percent` (`KismetMathLibrary.NormalizeToRange` (`/Game/Fire_Fight/BPC_damageable.CurrentHealth` _bpc_damageable) (`/Game/Fire_Fight/BPC_damageable.MaxHealth` _bpc_damageable)) _asw_civ_ui))))
    (:`then_1`
      ;[1 0.09711 0] take damage
      (if (`/Game/Fire_Fight/BPC_damageable.isDead` (`self.BPC_damageable`))
        (`self.CivilianDie`)))
    (:`then_2`
      ;[1 1 1] always correct rotation
      (if (not (`self.Carried`))
        (`SceneComponent.K2_SetRelativeRotation` _sphere (`KismetMathLibrary.MakeRotator` 0.0 0.0 _relativerotation_yaw) false false)))))

(event `self.Sphere.OnComponentBeginOverlap`
  (params (OverlappedComponent :type "PrimitiveComponent Object Reference") (OtherActor :type "Actor Object Reference") (OtherComp :type "PrimitiveComponent Object Reference") (OtherBodyIndex :type Integer) (bFromSweep :type Boolean) (SweepResult :type "HitResult Structure (by ref)"))
  (`|ExecutionSequence`
    (:`then_0`
      ;[0.2026 1 0.2461] save civilian
      (if (and (not (`/Game/Fire_Fight/BPC_damageable.isDead` (`self.BPC_damageable`))) (`KismetSystemLibrary.DoesImplementInterface` OtherActor "/Game/Fire_Fight/Characters/civilians/i_civSafePoint.i_civSafePoint_C"))
        (message `/Game/Fire_Fight/Characters/civilians/i_civSafePoint.civilian placed in safe spot` OtherActor)
        (`self.CivilianSaved`)
        (`self.K2_DetachFromActor` "KeepRelative")
        (`self.K2_AttachToActor` OtherActor "None" "SnapToTarget" "KeepRelative" "KeepWorld")
        (`KismetSystemLibrary.Delay` 0.5)
        (`/Game/Fire_Fight/Interactions/bpc_interact.display ui` (`self.bpc_interactCOMP`) false)
        (`SkeletalMeshComponent.PlayAnimation` (`self.person`) "/Game/Fire_Fight/Characters/civilians/animations/ue4_Joyful_Jump.ue4_Joyful_Jump" true)
        (`KismetSystemLibrary.Delay` 10.0)
        (`self.SetActorHiddenInGame` true)))))

(event `self.ui Overlap.OnComponentBeginOverlap`
  (params (OverlappedComponent :type "PrimitiveComponent Object Reference") (OtherActor :type "Actor Object Reference") (OtherComp :type "PrimitiveComponent Object Reference") (OtherBodyIndex :type Integer) (bFromSweep :type Boolean) (SweepResult :type "HitResult Structure (by ref)"))
  ;[1 0.4527 0] ui interaction
  (if (and (not (`/Game/Fire_Fight/BPC_damageable.isDead` (`self.BPC_damageable`))) (not (`self.CivilianSafe`)))
    (`/Game/Fire_Fight/Interactions/bpc_interact.display widget on overlap` (`self.bpc_interactCOMP`) OtherActor (`self.Carried`) true)))

(event `self.ui Overlap.OnComponentEndOverlap`
  (params (OverlappedComponent :type "PrimitiveComponent Object Reference") (OtherActor :type "Actor Object Reference") (OtherComp :type "PrimitiveComponent Object Reference") (OtherBodyIndex :type Integer))
  (`/Game/Fire_Fight/Interactions/bpc_interact.display widget on overlap` (`self.bpc_interactCOMP`) OtherActor false false))

(event `/Game/Fire_Fight/Characters/civilians/I_Civilian.CivilianDie`
  (bind _returnvalue (`WidgetComponent.GetWidget` (`self.dead widget`)))
  ;[1 0 0.01104] died :(
  (`|ExecutionSequence`
    (:`then_0`
      (`PrimitiveComponent.SetMaterial` (`self.Sphere`) 0 "/Game/Fire_Fight/Characters/civilians/materials/M_CivilianDie.M_CivilianDie")
      (`PrimitiveComponent.SetCollisionEnabled` (`self.Sphere`) "NoCollision")
      (bind _returnvalue_2 (`GameplayStatics.GetActorOfClass` "/Game/Fire_Fight/Assets/BP_GameManager.BP_GameManager_C"))
      (message `/Game/Fire_Fight/I_GameManager.CivilianDeath` _returnvalue_2)
      (`self.K2_DetachFromActor` "KeepWorld" "KeepWorld" "KeepWorld")
      (`PrimitiveComponent.SetSimulatePhysics` (`self.person`) true)
      (`PrimitiveComponent.SetCollisionObjectType` (`self.person`) "ECC_Pawn")
      (`/Engine/EditorBlueprintResources/StandardMacros.IsValid` _returnvalue
        (:`Is Valid`
          (bind _asw_civ_ui (cast `/Game/Fire_Fight/joost/civilians_UI/W_CivUI` _returnvalue))
          (`KismetSystemLibrary.Delay` 0.3)
          (set `/Game/Fire_Fight/joost/civilians_UI/W_CivUI.origin location` (`self.K2_GetActorLocation`) _asw_civ_ui))))
    (:`then_1`
      (if (`self.juiceON`)
        (`SceneComponent.SetVisibility` (`self.checpoint widget`) false false)
        (`SceneComponent.SetVisibility` (`self.dead widget`) true false)))
    (:`then_2`
      (`self.play dialogue` 4))))

(event `self.dialogue sphere.OnComponentBeginOverlap`
  (params (OverlappedComponent :type "PrimitiveComponent Object Reference") (OtherActor :type "Actor Object Reference") (OtherComp :type "PrimitiveComponent Object Reference") (OtherBodyIndex :type Integer) (bFromSweep :type Boolean) (SweepResult :type "HitResult Structure (by ref)"))
  ;[0 0.5221 1] dialogue settings
  (if (and (not (`self.Carried`)) (not (`/Game/Fire_Fight/BPC_damageable.isDead` (`self.BPC_damageable`))) (`KismetSystemLibrary.DoesImplementInterface` OtherActor "/Game/Fire_Fight/Characters/main_char/i_player.i_player_C") (not (`self.CivilianSafe`)))
    (if (or (not (`self.intro dialogue spoken`)) (`KismetMathLibrary.RandomBoolWithWeight` 0.25))
      (set `self.intro dialogue spoken` true)
      (`self.play dialogue` 1))))

(event `self.dialogue sphere.OnComponentEndOverlap`
  (params (OverlappedComponent :type "PrimitiveComponent Object Reference") (OtherActor :type "Actor Object Reference") (OtherComp :type "PrimitiveComponent Object Reference") (OtherBodyIndex :type Integer))
  ;[0 0.5221 1] dialogue settings
  (if (and (not (`self.Carried`)) (not (`/Game/Fire_Fight/BPC_damageable.isDead` (`self.BPC_damageable`))) (`KismetSystemLibrary.DoesImplementInterface` OtherActor "/Game/Fire_Fight/Characters/main_char/i_player.i_player_C") (not (`self.CivilianSafe`)))
    (`self.play dialogue` 0)))

(fn `carry person`
  (returns (`is being carried` :type Boolean))
  (`PrimitiveComponent.SetRenderCustomDepth` (`self.person`) true)
  (`SkeletalMeshComponent.SetAnimation` (`self.person`) "/Game/Fire_Fight/Characters/civilians/animations/ue4_rescuePose.ue4_rescuePose")
  (bind _output_get (set `self.Carried` true))
  (`self.play dialogue` 2)
  (`/Game/Fire_Fight/Interactions/bpc_interact.display ui` (`self.bpc_interactCOMP`) false)
  (return _output_get))

(fn `character get up`
  (bind _person (`self.person`))
  (bind _returnvalue (`SceneComponent.GetSocketLocation` _person "pelvis"))
  (if (not (`/Game/Fire_Fight/BPC_damageable.isDead` (`self.BPC_damageable`)))
    (bind (_outhit _returnvalue_2) (`KismetSystemLibrary.LineTraceSingle` _returnvalue (+ _returnvalue (* (`KismetMathLibrary.GetRightVector` (`SceneComponent.GetSocketRotation` _person "pelvis")) 50.0)) "TraceTypeQuery1"))
    (if _returnvalue_2
      (`KismetSystemLibrary.PrintString` "on front")
      (else
        (`KismetSystemLibrary.PrintString` "on back")))))

(fn `check bools`
  (returns (`is being carried` :type Boolean) (`is safe` :type Boolean))
  (return (`self.Carried`) (`self.CivilianSafe`)))

(fn `play dialogue`
  (params (`dialogue to play` :type Integer))
  (`AudioParameterControllerInterface.SetIntParameter` (`self.dialogue`) "dialogueCue" `dialogue to play`)
  (`AudioComponent.Play` (`self.dialogue`) 0.0)
  (return))

(fn `put down person`
  (returns (`is being carried` :type Boolean))
  (bind _person (`self.person`))
  (bind (_returnvalue_x _returnvalue_y) (`KismetMathLibrary.BreakVector` (`SceneComponent.K2_GetComponentLocation` _person)))
  (`self.K2_DetachFromActor` "KeepWorld" "KeepWorld" "KeepWorld")
  (bind _outhit (`KismetSystemLibrary.LineTraceSingle` (`SceneComponent.K2_GetComponentLocation` _person) (`KismetMathLibrary.MakeVector` _returnvalue_x _returnvalue_y -10000.0) "TraceTypeQuery1"))
  (`self.K2_SetActorLocation` (`.Location` (`GameplayStatics.BreakHitResult` _outhit)) true true)
  (`PrimitiveComponent.SetRenderCustomDepth` (`self.person`) true)
  (`SkeletalMeshComponent.PlayAnimation` (`self.person`) (select `bool` (`self.CivilianSafe`) :`false` "/Game/Fire_Fight/Characters/civilians/animations/ue4_Waving.ue4_Waving" :`true` "/Game/Fire_Fight/Characters/civilians/animations/ue4_Joyful_Jump.ue4_Joyful_Jump" :!type "AnimationAsset Object Reference") true)
  (if (`/Game/Fire_Fight/BPC_damageable.isDead` (`self.BPC_damageable`))
    _
    (else
      _))
  (bind _output_get (set `self.Carried` false))
  (`/Game/Fire_Fight/Interactions/bpc_interact.display ui` (`self.bpc_interactCOMP`) (not (`self.CivilianSafe`)))
  (return _output_get))

(fn `throw person`
  (returns (`is being carried` :type Boolean)))

(fn `UserConstructionScript`
  (`SceneComponent.SetVisibility` (`self.dead widget`) false false)
  (set `/Game/Fire_Fight/Interactions/bpc_interact.ui prompt` (`self.interaction UI`) (`self.bpc_interactCOMP`)))
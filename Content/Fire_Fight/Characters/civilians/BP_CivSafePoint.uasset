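; BP_CivSafePoint is a safe-spot marker for civilians, with a rotating cylinder and a toggleable SafePoint icon.
; CivilianPlacedinSafeSpot flashes the cylinder material, waits, then plays a timeline that enlarges EffectSpot from its current scale on each update.
; When the timeline finishes, it restores the normal material and sets EffectSpot to the cylinder scale cached in the construction script.
; The cylinder's overlap event is empty, so placement detection is not handled here.
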(event `/Game/Fire_Fight/Characters/civilians/i_civSafePoint.civilian placed in safe spot`
  (bind _effectspot (`self.EffectSpot`))
  (bind _relativescale3d (`SceneComponent.RelativeScale3D` _effectspot))
  (`PrimitiveComponent.SetMaterial` (`self.Cylinder`) 0 "/Game/Fire_Fight/Characters/civilians/materials/M_CivSafe_flash.M_CivSafe_flash")
  (`KismetSystemLibrary.Delay` 1.5)
  (bind (_direction _saved_effect) (`Timeline|efffect timeline` :!via `PlayFromStart`)
    (:`Update`
      (`SceneComponent.SetRelativeScale3D` _effectspot (`KismetMathLibrary.VLerp` _relativescale3d (* _relativescale3d 3.0) _saved_effect)))
    (:`Finished`
      (`PrimitiveComponent.SetMaterial` (`self.Cylinder`) 0 "/Game/Fire_Fight/Characters/civilians/materials/M_CivSafe.M_CivSafe")
      (`SceneComponent.SetRelativeScale3D` (`self.EffectSpot`) (`self.cylinder scale`)))))

(event `self.Cylinder.OnComponentBeginOverlap`
  (params (OverlappedComponent :type "PrimitiveComponent Object Reference") (OtherActor :type "Actor Object Reference") (OtherComp :type "PrimitiveComponent Object Reference") (OtherBodyIndex :type Integer) (bFromSweep :type Boolean) (SweepResult :type "HitResult Structure (by ref)")))

(event `self.ReceiveBeginPlay`
  (`MovementComponent.SetUpdatedComponent` (`self.RotatingMovement`) (`self.Cylinder`)))

(event `/Game/Fire_Fight/Characters/civilians/i_civSafePoint.Show icon`
  (params (OnOff :type Boolean))
  (`SceneComponent.SetVisibility` (`self.safe point`) OnOff false))

(fn `UserConstructionScript`
  (set `self.cylinder scale` (`SceneComponent.RelativeScale3D` (`self.Cylinder`))))
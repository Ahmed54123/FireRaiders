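; Inventory component for the Fire_Fight main character, tracking item counts in a map keyed by item.
; AddItem adds to an item's count, CheckAvailable reports whether any stock remains, and UsePlayerItem decrements one-time items without checking stock itself.
; UseItemDep combines check and use in one function, apparently a deprecated version.
; The check and use functions ignore their Quantity input and print debug text.
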(fn `Add Item`
  (params (Item :type "/Game/Fire_Fight/Assets/EquippableItems/PlayerItem_DataAsset Object Reference") (Quantity :type Integer))
  (`BlueprintMapLibrary.Map_Add` (`self.inventory`) Item (+ Quantity (`BlueprintMapLibrary.Map_Find` (`self.inventory`) Item))))

(fn `Check Available`
  (params (Item :type "/Game/Fire_Fight/Assets/EquippableItems/PlayerItem_DataAsset Object Reference") (Quantity :type Integer :default 1))
  (returns (`Available?` :type Boolean))
  (locals (`Player Item ` :type "/Game/Fire_Fight/Assets/EquippableItems/PlayerItem_DataAsset Object Reference"))
  (bind _returnvalue (> (`BlueprintMapLibrary.Map_Find` (`self.inventory`) Item) 0))
  (set `local.Player Item ` Item)
  ;[1 1 1] check if item is available
  (if (not _returnvalue)
    (`KismetSystemLibrary.PrintText` "out of stock"))
  (return _returnvalue))

(fn `Use Item (dep)`
  (params (Item :type "/Game/Fire_Fight/Assets/EquippableItems/PlayerItem_DataAsset Object Reference") (Quantity :type Integer :default 1))
  (locals (`Player Item ` :type "/Game/Fire_Fight/Assets/EquippableItems/PlayerItem_DataAsset Object Reference"))
  (set `local.Player Item ` Item)
  ;[1 1 1] check if item is available
  (if (> (`BlueprintMapLibrary.Map_Find` (`self.inventory`) Item) 0)
    (if (`/Game/Fire_Fight/Assets/EquippableItems/PlayerItem_DataAsset.One Time?` Item)
      ;[1 1 1] if the item can only be used once
      (`BlueprintMapLibrary.Map_Add` (`self.inventory`) (`local.Player Item `) (- (`BlueprintMapLibrary.Map_Find` (`self.inventory`) (`local.Player Item `)) 1))
      (`KismetSystemLibrary.PrintText` "used ability"))
    (else
      (`KismetSystemLibrary.PrintText` "out of stock"))))

(fn `Use Player Item`
  (params (Item :type "/Game/Fire_Fight/Assets/EquippableItems/PlayerItem_DataAsset Object Reference") (Quantity :type Integer :default 1))
  (locals (`Player Item ` :type "/Game/Fire_Fight/Assets/EquippableItems/PlayerItem_DataAsset Object Reference"))
  (set `local.Player Item ` Item)
  (if (`/Game/Fire_Fight/Assets/EquippableItems/PlayerItem_DataAsset.One Time?` Item)
    ;[1 1 1] if the item can only be used once
    (`BlueprintMapLibrary.Map_Add` (`self.inventory`) (`local.Player Item `) (- (`BlueprintMapLibrary.Map_Find` (`self.inventory`) (`local.Player Item `)) 1))
    (`KismetSystemLibrary.PrintText` "used ability")))
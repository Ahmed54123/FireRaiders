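; A Blueprint component that gives its owner health that can be damaged and healed.
; On BeginPlay it sets current health to max health.
; Damage and heal functions adjust health clamped between zero and max, and damage reaching zero sets a dead flag.
; Nothing in the component reacts to death or clears that flag.
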(event `self.ReceiveBeginPlay`
  (set `self.CurrentHealth` (`self.MaxHealth`)))

(fn `AddHealthFunc`
  (params (HealthApplied :type "Float (double-precision)"))
  (set `self.CurrentHealth` (`KismetMathLibrary.FClamp` (+ (`self.CurrentHealth`) HealthApplied) 0.0 (`self.MaxHealth`))))

(fn `TakeDamageFunc`
  (params (damageApplied :type "Float (double-precision)"))
  (bind _output_get (set `self.CurrentHealth` (`KismetMathLibrary.FClamp` (- (`self.CurrentHealth`) damageApplied) 0.0 (`self.MaxHealth`))))
  (if (<= _output_get 0.0)
    (set `self.isDead` true)))
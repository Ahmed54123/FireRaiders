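; Fire sprinkler actor that, when activated, extinguishes burning actors within its water collision volume for a set time.
; Construction caches the collision's authored scale, then hides it at zero scale with collision disabled.
; Activation optionally fades in sound and grows the volume through a rate-adjusted timeline, sending overlapped actors a stop-burning message with the extinguisher type.
; After a delay, it collapses the volume and fades out the sound.
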(event `self.ReceiveBeginPlay`
  (`AudioComponent.SetPaused` (`self.soundFX`) true))

(event `/Game/Fire_Fight/Interactions/I_Activated.ActivateFunction`
  (bind _sprinkler_water (`self.Sprinkler Water`))
  (bind _soundfx (`self.soundFX`))
  (`|ExecutionSequence`
    (:`then_0`
      (if (`self.SoundOn`)
        (`AudioComponent.SetPaused` _soundfx false)
        (`AudioComponent.FadeIn` _soundfx 0.5 1.0 0.0 "Linear")))
    (:`then_1`
      (`PrimitiveComponent.SetCollisionEnabled` (`self.Sprinker_Collision`) "QueryOnly")
      (`TimelineComponent.SetPlayRate` _sprinkler_water (/ (`TimelineComponent.GetTimelineLength` _sprinkler_water) (`self.SprinklerGrowRate`)))
      (bind (_direction _sprinkle) (`Timeline|Sprinkler Water`)
        (:`Update`
          (`SceneComponent.SetRelativeScale3D` (`self.Sprinker_Collision`) (`KismetMathLibrary.VLerp` (0.0 0.0 0.0) (`self.WaterCollSize`) _sprinkle)))
        (:`Finished`
          (`KismetSystemLibrary.Delay` (`self.Sprinkler time`))
          (`self.Turn Sprinklers Off`)
          (`AudioComponent.FadeOut` (`self.soundFX`) 0.5 0.0 "Linear"))))))

(event `self.Sprinker_Collision.OnComponentBeginOverlap`
  (params (OverlappedComponent :type "PrimitiveComponent Object Reference") (OtherActor :type "Actor Object Reference") (OtherComp :type "PrimitiveComponent Object Reference") (OtherBodyIndex :type Integer) (bFromSweep :type Boolean) (SweepResult :type "HitResult Structure (by ref)"))
  (message `/Game/Fire_Fight/Fire_Fire/I_Burnable.StopBurning` OtherActor (`/Game/Fire_Fight/Fire_Fire/fire_variants/bpc_ExtinguishComponent.Type` (`self.Extinguish Component`))))

(fn `Turn Sprinklers Off`
  (`SceneComponent.SetRelativeScale3D` (`self.Sprinker_Collision`) (0.0 0.0 0.0))
  (`PrimitiveComponent.SetCollisionEnabled` (`self.Sprinker_Collision`) "NoCollision"))

(fn `UserConstructionScript`
  (bind _sprinker_collision (`self.Sprinker_Collision`))
  (`PrimitiveComponent.SetCollisionEnabled` (`self.Sprinker_Collision`) "NoCollision")
  (set `self.WaterCollSize` (`SceneComponent.RelativeScale3D` _sprinker_collision))
  (`SceneComponent.SetRelativeScale3D` _sprinker_collision (0.0 0.0 0.0)))
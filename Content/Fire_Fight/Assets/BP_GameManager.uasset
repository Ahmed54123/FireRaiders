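; BP_GameManager runs a Fire_Fight level, tracking civilians and collectible badges and driving the objective HUD, level title and music.
; Counter events feed win and loss checks: a civilian death shows DeathScreen and reloads the level, while saving all civilians sets GameWinner.
; Tick polls these flags to update game-over UI and either load NextLevel after slow motion or, with ActivateDoor set, activate ActivateObjects instead.
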(event `self.ReceiveTick`
  (params (DeltaSeconds :type "Float (single-precision)"))
  (`|ExecutionSequence`
    (:`then_0`
      (if (`self.isGameOver`)
        ;[0.01771 0 1] once level conditions met, what to load next
        (`/Game/Fire_Fight/Assets/pickups/WB_GameHUD.game over UI` (`self.HUD Objectives`))))
    (:`then_1`
      (if (`self.GameWinner`)
        (if (not (`self.ActivateDoor?`))
          (bind _returnvalue (`GameplayStatics.GetActorOfClass` "/Game/Fire_Fight/Characters/main_char/BP_Nuri_FireRaider.BP_Nuri_FireRaider_C"))
          (`KismetSystemLibrary.Delay` 0.3)
          (`GameplayStatics.SetGlobalTimeDilation` 0.3)
          (message `/Game/Fire_Fight/Characters/main_char/i_player.Game Won` _returnvalue)
          (`KismetSystemLibrary.Delay` 4.0)
          (`GameplayStatics.OpenLevelBySoftObjectPtr` (`self.nextLevel`))
          (else
            (for _array_element (`self.activateObjects`)
              (message `/Game/Fire_Fight/Interactions/I_Activated.ActivateFunction` _array_element))))))))

(event `/Game/Fire_Fight/I_GameManager.AddCivilian`
  ;[1 0.6276 0] civilian logic
  (set `self.NumberOfCivilians` (+ (`self.NumberOfCivilians`) 1)))

(event `/Game/Fire_Fight/I_GameManager.CivilianDeath`
  ;[1 0.6276 0] civilian logic
  (set `self.CiviliansSaved` (- (`self.CiviliansSaved`) 1))
  (`/Game/Fire_Fight/I_GameManager.GameOver` "A Civilian Died"))

(event `/Game/Fire_Fight/I_GameManager.GameOver`
  (params (Reason :type String))
  (bind _game_music (`self.Game Music`))
  ;[0.1367 1 0.04177] win conditions
  (if (not (`self.isGameOver`))
    (set `self.isGameOver` true)
    (`GameplayStatics.GetActorOfClass` "/Game/Fire_Fight/Characters/main_char/BP_Nuri_FireRaider.BP_Nuri_FireRaider_C")
    (`AudioComponent.SetSound` _game_music "/Game/Fire_Fight/joost/sound_FX/music/music_v1/DefeatAudio__1_.DefeatAudio__1_")
    (`AudioComponent.Play` _game_music 0.0)
    (bind _returnvalue (`|CreateWidget` "/Game/Fire_Fight/Characters/main_char/playerHealth/DeathScreen.DeathScreen_C"))
    (`UserWidget.AddToViewport` _returnvalue 0)
    (`self.DisableInput` (`GameplayStatics.GetPlayerController` 0))
    (`/Game/Fire_Fight/Characters/main_char/playerHealth/DeathScreen.Show Game Over` _returnvalue Reason)
    (`KismetSystemLibrary.Delay` (`self.delay till next level`))
    (bind _returnvalue_2 (`GameplayStatics.GetCurrentLevelName` true))
    (`GameplayStatics.OpenLevel` (`KismetStringLibrary.Conv_StringToName` _returnvalue_2))))

(event `/Game/Fire_Fight/I_GameManager.CivilianSaved`
  ;[1 0.6276 0] civilian logic
  (bind _output_get (set `self.CiviliansSaved` (+ (`self.CiviliansSaved`) 1)))
  (`self.set civilian count in HUD`)
  (if (and (not (`self.isGameOver`)) (>= _output_get (`self.NumberOfCivilians`)))
    (`self.GameWon`)))

(event `/Game/Fire_Fight/I_GameManager.GameWon`
  (bind _game_music (`self.Game Music`))
  ;[0.1367 1 0.04177] win conditions
  (set `self.isGameOver` true)
  (set `self.GameWinner` true)
  (if (not (`self.ActivateDoor?`))
    (bind _outactors (`GameplayStatics.GetAllActorsWithInterface` "/Game/Fire_Fight/Characters/main_char/i_player.i_player_C"))
    (for _array_element _outactors
      (message `/Game/Fire_Fight/Characters/main_char/i_player.Game Won` _array_element))
    (`/Game/Fire_Fight/Assets/pickups/WB_GameHUD.Win Screen Anim` (`self.HUD Objectives`))
    (`AudioComponent.SetSound` _game_music "/Game/Fire_Fight/joost/sound_FX/music/Fire_Raiders_Theme_1.Fire_Raiders_Theme_1")
    (`AudioComponent.Play` _game_music 0.0)))

(event `/Game/Fire_Fight/I_GameManager.AddCollectible`
  ;[0.4009 0 1] collectibles
  (bind _output_get (set `self.Collectibles Picked` (+ (`self.Collectibles Picked`) 1)))
  (set `TextBlock.Text` (`KismetTextLibrary.Conv_StringToText` (`KismetStringLibrary.Concat_StrStr` (`KismetStringLibrary.Conv_IntToString` _output_get) "/" (`KismetStringLibrary.Conv_IntToString` (stale `/Game/Fire_Fight/I_GameManager.CountCollectibles` _output_get)) " Fire Badges")) (`/Game/Fire_Fight/Assets/pickups/WB_GameHUD.Collectibletext` (stale `self.ReceiveBeginPlay` _output_get)))
  (`/Game/Fire_Fight/Assets/pickups/WB_GameHUD.Play notification animation` (stale `self.ReceiveBeginPlay` _output_get)))

(event `/Game/Fire_Fight/I_GameManager.CountCollectibles`
  ;[0.4009 0 1] collectibles
  (bind _output_get (set `self.Collectibles in Game` (+ (`self.Collectibles in Game`) 1))))

(event `self.ReceiveBeginPlay`
  (bind _game_music (`self.Game Music`))
  ;[0.4009 0 1] collectibles
  (`|ExecutionSequence`
    (:`then_0`
      (bind _returnvalue (`|CreateWidget` "/Game/Fire_Fight/Assets/pickups/WB_GameHUD.WB_GameHUD_C"))
      (bind _output_get (set `self.HUD Objectives` _returnvalue))
      (`UserWidget.AddToViewport` _returnvalue 10)
      (`self.set objective in HUD`))
    (:`then_1`
      (`/Game/Fire_Fight/Assets/pickups/WB_GameHUD.Play Level Title Animation` (`self.HUD Objectives`) (`self.Level Titile`) (`self.Level Location`)))
    (:`then_2`
      (`AudioComponent.SetSound` _game_music (`self.Music`))
      (`AudioComponent.Play` _game_music 0.0))))

(fn `UserConstructionScript`)
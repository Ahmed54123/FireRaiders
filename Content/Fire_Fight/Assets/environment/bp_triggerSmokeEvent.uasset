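; Trigger actor that starts a smoke event by spawning BP_SmokeManager when the player character overlaps it.
; On BeginPlay it hides its Cube component and every actor in ActorsAffected; nothing here unhides those actors or passes them to the manager.
; The manager spawns at the trigger's transform, and the trigger then destroys itself, so it fires only once.
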(event `self.ReceiveBeginPlay`
  (`SceneComponent.SetHiddenInGame` (`self.Cube`) true false)
  (for _array_element (`self.actors affected`)
    (`self.SetActorHiddenInGame` _array_element true)))

(event `self.ReceiveActorBeginOverlap`
  (params (OtherActor :type "Actor Object Reference"))
  (if (== OtherActor (`GameplayStatics.GetPlayerCharacter` 0))
    (`|SpawnActorFromClass` "/Game/Fire_Fight/Fire_Fire/smoke/BP_SmokeManager.BP_SmokeManager_C" (`self.GetTransform`) "Undefined" "OverrideRootScale" null null)
    (`self.K2_DestroyActor`)))

(fn `UserConstructionScript`)
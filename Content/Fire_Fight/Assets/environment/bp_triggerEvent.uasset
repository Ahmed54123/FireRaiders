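; A trigger actor that reveals a set of hidden actors when the player walks into it.
; On BeginPlay it hides its Cube component and every actor in the ActorsAffected array.
; When player character 0 overlaps it, it loops over that array to unhide each actor, calling DestroyActor on itself inside the loop body, so it works as a one-shot.
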(event `self.ReceiveBeginPlay`
  (`SceneComponent.SetHiddenInGame` (`self.Cube`) true false)
  (for _array_element (`self.actors affected`)
    (`self.SetActorHiddenInGame` _array_element true)))

(event `self.ReceiveActorBeginOverlap`
  (params (OtherActor :type "Actor Object Reference"))
  (if (== OtherActor (`GameplayStatics.GetPlayerCharacter` 0))
    (for _array_element (`self.actors affected`)
      (`self.SetActorHiddenInGame` _array_element false)
      (`self.K2_DestroyActor`))))

(fn `UserConstructionScript`)
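; Throwable grenade that puts out fires by sending a StopBurning message to actors overlapping its extinguish radius.
; Throw runs once, detaching the grenade, launching it by projectile movement with a random tumble and soon starting its particles.
; It then hands its velocity to physics simulation and later enables the radius, which starts collision-free.
; GrenadeLifetime times the particle shutoff and the life span set afterward.
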(event `self.ReceiveBeginPlay`)

(event `Throw`
  (params (Velocity :type "Vector Structure"))
  (bind _main_collision (`self.main collision`))
  (bind _projectilemovement (`self.ProjectileMovement`))
  (`/Engine/EditorBlueprintResources/StandardMacros.DoOnce` false
    (:`Completed`
      (`|ExecutionSequence`
        (:`then_0`
          (`self.K2_DetachFromActor` "KeepWorld" "KeepWorld" "KeepWorld")
          (`KismetSystemLibrary.Delay` 0.2)
          (`ActorComponent.Activate` (`self.explosion particles`) false))
        (:`then_1`
          (set `MovementComponent.Velocity` Velocity _projectilemovement)
          (`ActorComponent.Activate` _projectilemovement false)
          (`KismetSystemLibrary.Delay` 0.4)
          (`PrimitiveComponent.SetCollisionEnabled` (`self.main collision`) "QueryAndPhysics")
          (bind _output_get (set `self.Velocity` (`self.GetVelocity`)))
          (`PrimitiveComponent.SetSimulatePhysics` _main_collision true)
          (`PrimitiveComponent.SetPhysicsLinearVelocity` _main_collision _output_get false "None")
          (`KismetSystemLibrary.Delay` 1.0)
          (`PrimitiveComponent.SetCollisionEnabled` (`self.extinguish radius`) "QueryOnly")
          (`KismetSystemLibrary.Delay` (- (`self.grenade lifetime`) 0.4))
          (`ActorComponent.Deactivate` (`self.explosion particles`))
          (`SceneComponent.SetHiddenInGame` (`self.mesh`) false false)
          (`self.SetLifeSpan` (`self.grenade lifetime`)))
        (:`then_2`
          (`KismetSystemLibrary.MoveComponentTo` (`self.mesh`) (0.0 0.0 0.0) (`KismetMathLibrary.RandomRotator` false) false false 0.5))))))

(event `self.extinguish radius.OnComponentBeginOverlap`
  (params (OverlappedComponent :type "PrimitiveComponent Object Reference") (OtherActor :type "Actor Object Reference") (OtherComp :type "PrimitiveComponent Object Reference") (OtherBodyIndex :type Integer) (bFromSweep :type Boolean) (SweepResult :type "HitResult Structure (by ref)"))
  (message `/Game/Fire_Fight/Fire_Fire/I_Burnable.StopBurning` OtherActor "NewEnumerator1"))

(fn `UserConstructionScript`
  (`PrimitiveComponent.SetCollisionEnabled` (`self.extinguish radius`) "NoCollision")
  (`PrimitiveComponent.SetCollisionEnabled` (`self.main collision`) "NoCollision"))
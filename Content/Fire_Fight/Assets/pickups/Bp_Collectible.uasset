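; Bp_Collectible is a pickup that grants health and ammo to actors implementing the I_player interface and counts toward the game's collectible total.
; On BeginPlay it registers itself with BP_GameManager through an interface message.
; On overlap it notifies the player and manager, plays CollectFX, sends health and ammo values, then hides itself and disables sphere collision instead of being destroyed.
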(event `self.ReceiveActorBeginOverlap`
  (params (OtherActor :type "Actor Object Reference"))
  (if (`KismetSystemLibrary.DoesImplementInterface` OtherActor "/Game/Fire_Fight/Characters/main_char/i_player.i_player_C")
    (message `/Game/Fire_Fight/Characters/main_char/i_player.Collectibe Collected` OtherActor)
    (bind _returnvalue (`GameplayStatics.GetActorOfClass` "/Game/Fire_Fight/Assets/BP_GameManager.BP_GameManager_C"))
    (message `/Game/Fire_Fight/I_GameManager.AddCollectible` _returnvalue)
    (`ActorComponent.Activate` (`self.collectFX`) false)
    (message `/Game/Fire_Fight/I_idamageable.AddHealth` OtherActor (`self.pickup health value`))
    (message `/Game/Fire_Fight/Characters/main_char/i_player.add ammo` OtherActor (`self.pickup ammo value`))
    (`self.SetActorHiddenInGame` true)
    (`PrimitiveComponent.SetCollisionEnabled` (`self.Sphere`) "NoCollision")))

(event `self.ReceiveBeginPlay`
  (bind _returnvalue (`GameplayStatics.GetActorOfClass` "/Game/Fire_Fight/Assets/BP_GameManager.BP_GameManager_C"))
  (message `/Game/Fire_Fight/I_GameManager.CountCollectibles` _returnvalue))

(fn `UserConstructionScript`)
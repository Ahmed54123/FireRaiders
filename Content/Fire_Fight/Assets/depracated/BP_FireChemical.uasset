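; BP_FireChemical is a chemical fire hazard that ignites on BeginPlay and can be put out by an extinguisher but not water.
; A timeline grows the fire cone at the BPFireProperties spread rate, with optional sound, smoke and "juice" effects.
; Cone overlaps ignite other actors through interface messages and start timer-driven damage.
; Extinguishing stops damage and effects and lowers the smoke manager's smoke amount.
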(event `/Game/Fire_Fight/Fire_Fire/I_Burnable.Start Burning`
  (params (`fire type` :type "/Game/Fire_Fight/Fire_Fire/fire_variants/e_FireType Enum" :default "NewEnumerator0") (`Spread Rate multiplier` :type "Float (double-precision)"))
  (bind _fire_cone (`self.fire Cone`))
  (bind _fire_spread (`self.Fire Spread`))
  (bind _bp_fireproperties (`self.BP_FireProperties`))
  (`/Engine/EditorBlueprintResources/StandardMacros.IsValid` _bp_fireproperties
    (:`Is Valid`
      (if (not (`/Game/Fire_Fight/Fire_Fire/BP_FireProperties.IsOnFire` _bp_fireproperties))
        (set `/Game/Fire_Fight/Fire_Fire/BP_FireProperties.IsOnFire` true _bp_fireproperties)
        (`|ExecutionSequence`
          (:`then_0`
            (if (`self.sound on`)
              (`AudioComponent.FadeIn` (`self.fireFX`) 1.5 1.0 0.0 "Linear")))
          (:`then_1`
            (if (`self.juice on`)
              (`ActorComponent.Activate` (`self.Ns_StylizedSmoke`) false)
              (`SceneComponent.SetVisibility` _fire_cone false false)
              (`ActorComponent.Activate` (`self.text effect`) false)
              (else
                (`SceneComponent.SetVisibility` _fire_cone true false))))
          (:`then_2`
            ;[1 0.439 0.04911] Make fire spread
            (if (`self.produces smoke`)
              (`/Game/Fire_Fight/Fire_Fire/BP_FireProperties.Produce Smoke` (`self.BP_FireProperties`)))
            (`TimelineComponent.SetPlayRate` _fire_spread (/ (`TimelineComponent.GetTimelineLength` _fire_spread) (`/Game/Fire_Fight/Fire_Fire/BP_FireProperties.SpreadRate` (`self.BP_FireProperties`))))
            (bind (_direction _fire_scale_change) (`Timeline|Fire Spread` :!via `PlayFromStart`)
              (:`Update`
                (`SceneComponent.SetRelativeScale3D` (`self.fire Cone`) (`KismetMathLibrary.VLerp` (0.0 0.0 0.0) (`self.fire Cone Size`) _fire_scale_change)))))
          (:`then_3`
            (`PrimitiveComponent.SetCollisionEnabled` (`self.fire Cone`) "QueryOnly")))))))

(event `self.fire Cone.OnComponentBeginOverlap`
  (params (OverlappedComponent :type "PrimitiveComponent Object Reference") (OtherActor :type "Actor Object Reference") (OtherComp :type "PrimitiveComponent Object Reference") (OtherBodyIndex :type Integer) (bFromSweep :type Boolean) (SweepResult :type "HitResult Structure (by ref)"))
  ;[1 1 1] Make objects take damage on overlap
  (`self.EventDamage`)
  (message `/Game/Fire_Fight/Fire_Fire/I_Burnable.Start Burning` OtherActor (`/Game/Fire_Fight/Fire_Fire/BP_FireProperties.fire type` (`self.BP_FireProperties`)) 1.0))

(event `self.ReceiveBeginPlay`
  (`SceneComponent.SetVisibility` (`self.fireMesh`) false false)
  (`self.Start Burning` "NewEnumerator0"))

(event `EventDamage`
  (bind _bp_fireproperties (`self.BP_FireProperties`))
  ;[1 0.0599 0.0599] Inflict damage on other object
  (if (`/Game/Fire_Fight/Fire_Fire/BP_FireProperties.IsOnFire` (`self.BP_FireProperties`))
    (for _array_element (`PrimitiveComponent.GetOverlappingActors` (`self.fire Cone`) null)
      (message `/Game/Fire_Fight/I_idamageable.takeDamage` _array_element (`/Game/Fire_Fight/Fire_Fire/BP_FireProperties.FireDamage` _bp_fireproperties))
      (bind _returnvalue (`KismetSystemLibrary.K2_SetTimerDelegate` (`|CreateDelegate` :!event `EventDamage`) (`/Game/Fire_Fight/Fire_Fire/BP_FireProperties.BurnRate` _bp_fireproperties) (`/Game/Fire_Fight/Fire_Fire/BP_FireProperties.IsOnFire` (`self.BP_FireProperties`)) false 0.05))
      (set `self.BurnerTimer` _returnvalue))))

(event `/Game/Fire_Fight/Fire_Fire/I_Burnable.StopBurning`
  (params (`object type` :type "/Game/Fire_Fight/Fire_Fire/fire_variants/e_FireExtinguishType Enum" :default "NewEnumerator0"))
  (bind _fire_spread (`self.Fire Spread`))
  ;[0.125 0.2349 1] stop the fire
  (if (select `/Game/Fire_Fight/Fire_Fire/fire_variants/e_FireExtinguishType` `object type` :`NewEnumerator1` true)
    (set `/Game/Fire_Fight/Fire_Fire/BP_FireProperties.IsOnFire` false (`self.BP_FireProperties`))
    (`KismetSystemLibrary.K2_ClearAndInvalidateTimerHandle` (`self.BurnerTimer`))
    (`TimelineComponent.Reverse` _fire_spread)
    (`TimelineComponent.SetNewTime` _fire_spread 0.0)
    (bind _returnvalue (`GameplayStatics.GetActorOfClass` "/Game/Fire_Fight/Fire_Fire/smoke/BP_SmokeManager.BP_SmokeManager_C"))
    (message `/Game/Fire_Fight/Fire_Fire/smoke/I_SmokeEvent.DecreaseSmokeAmount` _returnvalue (`self.smoke decrease amount`))
    (`AudioComponent.FadeOut` (`self.fireFX`) 1.4 0.0 "Linear")
    (`ActorComponent.Deactivate` (`self.Ns_StylizedSmoke`))
    (`PrimitiveComponent.SetCollisionEnabled` (`self.fire Cone`) "NoCollision")))

(event `/Game/Fire_Fight/Fire_Fire/I_Burnable.FireDieOut`
  ;[0.1224 0.1224 0.1224] Fire die out
  (set `/Game/Fire_Fight/Fire_Fire/BP_FireProperties.IsOnFire` false (`self.BP_FireProperties`))
  (`KismetSystemLibrary.K2_ClearAndInvalidateTimerHandle` (`self.BurnerTimer`))
  (`self.SetActorHiddenInGame` true)
  (`ActorComponent.Deactivate` (`self.Ns_StylizedSmoke`))
  (`PrimitiveComponent.SetCollisionEnabled` (`self.fire Cone`) "NoCollision"))

(fn `ApplyBurnDamage`
  (params (Damage :type "Float (double-precision)") (BurnTarget :type "Actor Object Reference"))
  (message `/Game/Fire_Fight/I_idamageable.takeDamage` BurnTarget Damage))

(fn `GetBurnRate`
  (returns (`Burn Rate` :type "Float (double-precision)"))
  (return 0.0))

(fn `GetMaterial`
  (returns (`Structure Type` :type "/Game/Fire_Fight/Fire_Fire/E_MaterialTypes Enum"))
  (return "NewEnumerator0"))

(fn `UserConstructionScript`
  (set `/Game/Fire_Fight/Fire_Fire/BP_FireProperties.IsOnFire` false (`self.BP_FireProperties`))
  (set `self.fire Cone Size` (`SceneComponent.RelativeScale3D` (`self.fire Cone`)))
  (`SceneComponent.SetRelativeScale3D` (`self.fire Cone`) (0.0 0.0 0.0)))
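; BP_BurnableBasicObject is a burnable prop, filed under deprecated assets, that can catch fire and burn out.
; StartBurning spawns fire at its spawn point through BPCBurnableProperties.
; TakeDamage scales damage by the fire multiplier into BPCDamageable, with brief invulnerability throttling hits; on death the cube gets a burnt material and the fire is told to die out once.
; GetBurnRate and GetMaterial return fixed defaults.
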(event `/Game/Fire_Fight/I_idamageable.takeDamage`
  (params (damage :type "Float (double-precision)"))
  (bind _bpc_burnableproperties (`self.BPC_BurnableProperties`))
  (if (not (`self.Invulnerable`))
    (`/Game/Fire_Fight/BPC_damageable.TakeDamageFunc` (`self.BPC_damageable`) (* damage (`/Game/Fire_Fight/Fire_Fire/BPC_BurnableProperties.fireEffectMultiplier` (`self.BPC_BurnableProperties`))))
    (set `self.Invulnerable` true)
    (`KismetSystemLibrary.Delay` 0.1)
    (set `self.invulnerable` false)
    (if (`/Game/Fire_Fight/BPC_damageable.isDead` (`self.BPC_damageable`))
      (`PrimitiveComponent.SetMaterial` (`self.Cube`) 0 "/Game/Fire_Fight/Materials/M_BurntObject.M_BurntObject")
      (if (not (`/Game/Fire_Fight/Fire_Fire/BPC_BurnableProperties.ObjectBurnt` _bpc_burnableproperties))
        (message `/Game/Fire_Fight/Fire_Fire/I_Burnable.FireDieOut` (`/Game/Fire_Fight/Fire_Fire/BPC_BurnableProperties.FireSpawn` _bpc_burnableproperties))
        (set `/Game/Fire_Fight/Fire_Fire/BPC_BurnableProperties.ObjectBurnt` true _bpc_burnableproperties)))))

(event `/Game/Fire_Fight/Fire_Fire/I_Burnable.Start Burning`
  (params (`fire type` :type "/Game/Fire_Fight/Fire_Fire/fire_variants/e_FireType Enum" :default "NewEnumerator0") (`Spread Rate multiplier` :type "Float (double-precision)"))
  (`/Game/Fire_Fight/Fire_Fire/BPC_BurnableProperties.SpawnFire` (`self.BPC_BurnableProperties`) (`self.fireSpawnPoint`) (`self.GetTransform`) "fire socket" "NewEnumerator0" 3.0))

(fn `GetBurnRate`
  (returns (`Burn Rate` :type "Float (double-precision)"))
  (return 0.0))

(fn `GetMaterial`
  (returns (`Structure Type` :type "/Game/Fire_Fight/Fire_Fire/E_MaterialTypes Enum"))
  (return "NewEnumerator0"))

(fn `UserConstructionScript`)
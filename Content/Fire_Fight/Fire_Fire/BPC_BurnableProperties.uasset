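; Actor component that makes an object burnable, managing the fire actor spawned on it in the firefighting game.
; On BeginPlay it picks a fire effect multiplier from the object's construction material type.
; SpawnFire spawns a normal or chemical fire on the first call and snaps it to a socket on the given component.
; Later calls message that fire to keep burning as normal fire at the given spread rate, or to die out once burnt.
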(event `self.ReceiveBeginPlay`
  (`self.CheckMaterialType`))

(fn `CheckMaterialType`
  (set `self.fireEffectMultiplier` (select `/Game/Fire_Fight/Fire_Fire/E_MaterialTypes` (`self.Material Type`) :`NewEnumerator0` (`self.FireResistive`) :`NewEnumerator1` (`self.OrdinaryConstruction`) :`NewEnumerator2` (`self.HeavyTimberSpreadRate`) :`NewEnumerator3` (`self.WoodFramingSpreadRate`))))

(fn `SpawnFire`
  (params (FireLocation :type "SceneComponent Object Reference") (`Actor location` :type "Transform Structure") (`socket name` :type Name) (`fire type` :type "/Game/Fire_Fight/Fire_Fire/fire_variants/e_FireType Enum" :default "NewEnumerator0") (`fire spread rate` :type "Float (double-precision)" :default 3.0))
  (locals (FireLocation :type "SceneComponent Object Reference") (`socket name` :type Name :default "None") (`fire spawn type` :type "/Game/Fire_Fight/Fire_Fire/fire_variants/e_FireType Enum" :default "NewEnumerator0"))
  (set `local.fire spawn type` `fire type`)
  (if (`self.ObjectBurnt`)
    (message `/Game/Fire_Fight/Fire_Fire/I_Burnable.FireDieOut` (`self.FireSpawn`))
    (elif (`self.FireSpawned`)
      (message `/Game/Fire_Fight/Fire_Fire/I_Burnable.Start Burning` (`self.FireSpawn`) "NewEnumerator0" `fire spread rate`)
      (else
        (set `self.FireSpawned` true)
        (bind _returnvalue (`|SpawnActorFromClass` (select `/Game/Fire_Fight/Fire_Fire/fire_variants/e_FireType` (`local.fire spawn type`) :`NewEnumerator0` "/Game/Fire_Fight/Fire_Fire/BP_FireMain.BP_FireMain_C" :`NewEnumerator1` "/Game/Fire_Fight/Fire_Fire/fire_variants/BP_FireChem.BP_FireChem_C" :!type "Actor Class Reference") `Actor location` "Undefined" "SelectDefaultAtRuntime" null null))
        (`Actor.K2_AttachToComponent` _returnvalue (`local.FireLocation`) (`local.socket name`) "SnapToTarget" "KeepWorld" "KeepWorld" true)
        (set `self.FireSpawn` _returnvalue)))))
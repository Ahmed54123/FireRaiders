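; Interactable window for a fire-fighting game that opens once to ventilate smoke.
; A trigger volume shows the prompt through BpcInteract; Interact hides it and the highlight circle, then runs the opening.
; Opening tells BP_SmokeManager to reduce smoke amount and apply a speed-decrease multiplier, starts wind effect and optional sound, and slides the window via timeline before hiding it.
; The construction script aims wind along WindDIRECTION's forward vector.
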(event `/Game/Fire_Fight/Interactions/I_Activated.ActivateFunction`
  (bind _window (`self.window`))
  (bind _window_2 (`self.window`))
  (bind _windsound (`self.WindSound`))
  (if (not (`self.alreadyOpened`))
    (`|ExecutionSequence`
      (:`then_0`
        (if (`self.SoundON`)
          (`AudioComponent.FadeIn` _windsound 0.2 1.0 0.0 "Linear")
          (`KismetSystemLibrary.Delay` 2.0)
          (`AudioComponent.FadeOut` _windsound 2.0 0.0 "Linear")))
      (:`then_1`
        (set `self.alreadyOpened` true)
        (bind _returnvalue (`GameplayStatics.GetActorOfClass` "/Game/Fire_Fight/Fire_Fire/smoke/BP_SmokeManager.BP_SmokeManager_C"))
        (message `/Game/Fire_Fight/Fire_Fire/smoke/I_SmokeEvent.DecreaseSmokeAmount` _returnvalue (`self.Amount ventilated`))
        (message `/Game/Fire_Fight/Fire_Fire/smoke/I_SmokeEvent.OpenWindow` _returnvalue (`self.speed decrease multiplier`))
        (`ActorComponent.Activate` (`self.wind effect`) false)
        (bind (_direction _open_window) (`Timeline|open window`)
          (:`Update`
            (`SceneComponent.K2_SetRelativeLocation` _window (`KismetMathLibrary.VLerp` (`SceneComponent.RelativeLocation` _window) (`SceneComponent.RelativeLocation` (`self.windowOpenPoint`)) _open_window) false false))
          (:`Finished`
            (`PrimitiveComponent.SetCollisionEnabled` _window_2 "NoCollision")
            (`SceneComponent.SetHiddenInGame` _window_2 true false)))))))

(event `/Game/Fire_Fight/Interactions/I_Interact.Interact`
  (`self.ActivateFunction`)
  (`SceneComponent.SetHiddenInGame` (`self.effectCircle`) true true)
  (`/Game/Fire_Fight/Interactions/bpc_interact.display ui` (`self.bpc_interact`) false))

(event `self.trigger spot.OnComponentBeginOverlap`
  (params (OverlappedComponent :type "PrimitiveComponent Object Reference") (OtherActor :type "Actor Object Reference") (OtherComp :type "PrimitiveComponent Object Reference") (OtherBodyIndex :type Integer) (bFromSweep :type Boolean) (SweepResult :type "HitResult Structure (by ref)"))
  (`/Game/Fire_Fight/Interactions/bpc_interact.display widget on overlap` (`self.bpc_interact`) OtherActor (`self.alreadyOpened`) true))

(event `self.trigger spot.OnComponentEndOverlap`
  (params (OverlappedComponent :type "PrimitiveComponent Object Reference") (OtherActor :type "Actor Object Reference") (OtherComp :type "PrimitiveComponent Object Reference") (OtherBodyIndex :type Integer))
  (`/Game/Fire_Fight/Interactions/bpc_interact.display widget on overlap` (`self.bpc_interact`) OtherActor (`self.alreadyOpened`) false))

(fn `UserConstructionScript`
  (`SceneComponent.SetRelativeScale3D` (`self.NS_Pulse`) (1.116767 1.116767 1.116767))
  (`NiagaraComponent.SetVariableVec3` (`self.wind effect`) "windDirectionLocal" (`SceneComponent.GetForwardVector` (`self.WindDIRECTION`)))
  (set `/Game/Fire_Fight/Interactions/bpc_interact.ui prompt` (`self.Widget`) (`self.bpc_interact`)))
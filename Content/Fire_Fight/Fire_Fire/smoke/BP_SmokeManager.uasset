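; BP_SmokeManager tracks the room's smoke level in the firefighting game and ends the game through BP_GameManager when it reaches the maximum.
; Other actors call events to add or remove smoke, while opening windows lowers the generation multiplier.
; On BeginPlay it enables volumetric fog and creates SmokeWidget, whose bar Tick updates with an interpolated, normalized smoke value.
; The construction script hides the SmokeCloud component.
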(event `self.ReceiveBeginPlay`
  (`|ExecutionSequence`
    (:`then_0`
      (bind _returnvalue (`GameplayStatics.GetActorOfClass` "/Script/Engine.ExponentialHeightFog"))
      (`/Engine/EditorBlueprintResources/StandardMacros.IsValid` _returnvalue
        (:`Is Valid`
          (`ExponentialHeightFogComponent.SetVolumetricFog` (`ExponentialHeightFog.Component` _returnvalue) true))))
    (:`then_1`
      ;[1 1 1] handle widget
      (bind _returnvalue_2 (`|CreateWidget` "/Game/Fire_Fight/Fire_Fire/smoke/SmokeWidget.SmokeWidget_C"))
      (set `self.SmokeWid` _returnvalue_2)
      (`UserWidget.AddToViewport` _returnvalue_2 0))))

(event `self.ReceiveTick`
  (params (DeltaSeconds :type "Float (single-precision)"))
  (bind _returnvalue (`KismetMathLibrary.FInterpTo` (`self.interp smoke`) (`self.SmokeLevel`) (`GameplayStatics.GetWorldDeltaSeconds`) 1.0))
  ;[1 1 1] handle widget
  (bind _assmoke_widget (cast `/Game/Fire_Fight/Fire_Fire/smoke/SmokeWidget` (`self.SmokeWid`)))
  (set `self.interp smoke` _returnvalue)
  (`ProgressBar.SetPercent` (`/Game/Fire_Fight/Fire_Fire/smoke/SmokeWidget.smokeBar` _assmoke_widget) (`KismetMathLibrary.FClamp` (- (`KismetMathLibrary.MapRangeClamped` _returnvalue 0.0 (`self.MaxSmoke`) 0.0 1.0) 0.12))))

(event `/Game/Fire_Fight/Fire_Fire/smoke/I_SmokeEvent.IncreaseSmokeAmount`
  (params (smokeAdded :type "Float (double-precision)"))
  ;[1 1 1] add smoke
  (if (not (`self.MaxSmokeReached`))
    (set `self.SmokeLevel` (+ (`self.SmokeLevel`) (* smokeAdded (`self.SmokeGenerationMultiplier`))))
    (if (>= (`self.SmokeLevel`) (`self.MaxSmoke`))
      (set `self.MaxSmokeReached` true)
      (bind _returnvalue (`GameplayStatics.GetActorOfClass` "/Game/Fire_Fight/Assets/BP_GameManager.BP_GameManager_C"))
      (message `/Game/Fire_Fight/I_GameManager.GameOver` _returnvalue "Smoke Filled the Area"))))

(event `/Game/Fire_Fight/Fire_Fire/smoke/I_SmokeEvent.DecreaseSmokeAmount`
  (params (`smoke decreased` :type "Float (double-precision)"))
  ;[1 1 1] decrease smoke
  (set `self.SmokeLevel` (- (`self.SmokeLevel`) `smoke decreased`)))

(event `/Game/Fire_Fight/Fire_Fire/smoke/I_SmokeEvent.OpenWindow`
  (params (`decrease amount` :type "Float (double-precision)"))
  (set `self.SmokeGenerationMultiplier` (`KismetMathLibrary.FClamp` (- (`self.SmokeGenerationMultiplier`) `decrease amount`))))

(fn `UserConstructionScript`
  (`SceneComponent.SetVisibility` (`self.SmokeCloud`) false false))
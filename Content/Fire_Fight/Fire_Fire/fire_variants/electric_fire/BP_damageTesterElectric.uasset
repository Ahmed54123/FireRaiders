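; BP_damageTesterElectric is a burnable electrical test actor that starts a fire at its cube's fire socket on play.
; While powered, Tick calls StartBurning after a half-second delay if the fire spawn is valid.
; ActivateFunction cuts power, after which Tick tells the fire to die out and deactivates the Electricity component.
; BPCBurnableProperties handles fire spawning, and the actor reports a zero burn rate and a fixed material type.
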(event `self.ReceiveBeginPlay`
  (`self.Start Burning` "NewEnumerator0"))

(event `self.ReceiveTick`
  (params (DeltaSeconds :type "Float (single-precision)"))
  (bind _poweron (`self.powerON`))
  (bind _firespawn (`/Game/Fire_Fight/Fire_Fire/BPC_BurnableProperties.FireSpawn` (`self.BPC_BurnableProperties`)))
  (`|ExecutionSequence`
    (:`then_0`
      (if _poweron
        (`/Engine/EditorBlueprintResources/StandardMacros.IsValid` (`/Game/Fire_Fight/Fire_Fire/BPC_BurnableProperties.FireSpawn` (`self.BPC_BurnableProperties`))
          (:`Is Valid`
            (`KismetSystemLibrary.Delay` 0.5)
            (`self.Start Burning` "NewEnumerator0")))
        (else
          (`/Engine/EditorBlueprintResources/StandardMacros.IsValid` _firespawn
            (:`Is Valid`
              (message `/Game/Fire_Fight/Fire_Fire/I_Burnable.FireDieOut` _firespawn))))))
    (:`then_1`
      (if (not _poweron)
        (`ActorComponent.Deactivate` (`self.electricity`))))))

(event `/Game/Fire_Fight/Fire_Fire/I_Burnable.Start Burning`
  (params (`fire type` :type "/Game/Fire_Fight/Fire_Fire/fire_variants/e_FireType Enum" :default "NewEnumerator0") (`Spread Rate multiplier` :type "Float (double-precision)"))
  (`/Game/Fire_Fight/Fire_Fire/BPC_BurnableProperties.SpawnFire` :`self` (`self.BPC_BurnableProperties`) :`FireLocation` (`self.Cube`) :`socket name` "fire socket"))

(event `/Game/Fire_Fight/Interactions/I_Activated.ActivateFunction`
  (set `self.powerON` false))

(fn `GetBurnRate`
  (returns (`Burn Rate` :type "Float (double-precision)"))
  (return 0.0))

(fn `GetMaterial`
  (returns (`Structure Type` :type "/Game/Fire_Fight/Fire_Fire/E_MaterialTypes Enum"))
  (return "NewEnumerator0"))

(fn `UserConstructionScript`)
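; BP_ResourceFire_prometheus is a resource fire variant that lights itself again whenever it is not burning.
; Tick polls IsOnFire on BPFireProperties and, when false, waits a FireLightTim delay before calling StartBurning with that component's FireType and an unmodified spread rate.
; The fire state is not rechecked after the delay, and the construction script only calls its parent.
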(event `self.ReceiveTick`
  (params (DeltaSeconds :type "Float (single-precision)"))
  (bind _bp_fireproperties (`self.BP_FireProperties`))
  (if (not (`/Game/Fire_Fight/Fire_Fire/BP_FireProperties.IsOnFire` _bp_fireproperties))
    (`KismetSystemLibrary.Delay` (`self.fireLightTim`))
    (`self.Start Burning` (`/Game/Fire_Fight/Fire_Fire/BP_FireProperties.fire type` _bp_fireproperties))))

(fn `UserConstructionScript`
  (`parent.UserConstructionScript`))
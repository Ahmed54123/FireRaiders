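; BP_FireChem is a chemical fire variant that can be put out by a fire extinguisher but not by water.
; Its StopBurning event clears the burn state and timer, reverses the FireSpread timeline and tells BP_SmokeManager to decrease smoke.
; It also fades out the fire, deactivates smoke and sound effects, and disables the fire cone's collision.
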(event `/Game/Fire_Fight/Fire_Fire/I_Burnable.StopBurning`
  (params (`object type` :type "/Game/Fire_Fight/Fire_Fire/fire_variants/e_FireExtinguishType Enum" :default "NewEnumerator0"))
  (bind _fire_spread (`self.Fire Spread`))
  (if (select `/Game/Fire_Fight/Fire_Fire/fire_variants/e_FireExtinguishType` `object type` :`NewEnumerator1` true)
    (set `/Game/Fire_Fight/Fire_Fire/BP_FireProperties.IsOnFire` false (`self.BP_FireProperties`))
    (`KismetSystemLibrary.K2_ClearAndInvalidateTimerHandle` (`self.BurnerTimer`))
    (`TimelineComponent.Reverse` _fire_spread)
    (`TimelineComponent.SetNewTime` _fire_spread 0.0)
    (bind _returnvalue (`GameplayStatics.GetActorOfClass` "/Game/Fire_Fight/Fire_Fire/smoke/BP_SmokeManager.BP_SmokeManager_C"))
    (message `/Game/Fire_Fight/Fire_Fire/smoke/I_SmokeEvent.DecreaseSmokeAmount` _returnvalue (`self.smoke decrease amount`))
    (`AudioComponent.FadeOut` (`self.fireFX`) 1.4 0.0 "Linear")
    (`ActorComponent.Deactivate` (`self.Ns_StylizedSmoke`))
    (`PrimitiveComponent.SetCollisionEnabled` (`self.fire Cone`) "NoCollision")
    (`self.deactivate particles`)))

(fn `UserConstructionScript`
  (`parent.UserConstructionScript`))